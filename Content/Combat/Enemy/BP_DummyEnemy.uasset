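; BP_DummyEnemy is a placeholder enemy for Dungeon Slayer combat, with a health value that incoming damage reduces.
; Any overlap with its Box component calls StartBattle on the DungeonSlayer game mode.
; It exposes combat functions for the battle flow: TakeDamage subtracts from Health, IsAlive reports Health above zero, ExecuteAction returns a fixed test string, and EnemyDead destroys the actor.
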(event OnComponentBeginOverlap(Box)
  (params (OverlappedComponent :type Primitive%20Component%20Object%20Reference) (OtherActor :type Actor%20Object%20Reference) (OtherComp :type Primitive%20Component%20Object%20Reference) (OtherBodyIndex :type Integer) (bFromSweep :type Boolean) (SweepResult :type Hit%20Result%20Structure%20%28by%20ref%29))
  (bind _asbp_dungeon_slayer_game_mode (Utilities|Casting|CastToBP_DungeonSlayerGameMode (Game|GetGameMode)))
  (Default|StartBattle _asbp_dungeon_slayer_game_mode))

(event EventBeginPlay)

(event Collision|EventActorBeginOverlap
  (params (OtherActor :type Actor%20Object%20Reference)))

(event EventTick
  (params (DeltaSeconds :type Float%20%28single-precision%29)))

(fn ConstructionScript)

(fn EnemyDead
  (Actor|DestroyActor)
  (return))

(fn ExecuteAction
  (return "I am enemy!!!"))

(fn IsAlive
  (Math|Integer|CompareInt (Variables|Default|GetHealth)
    (:>
      (return true))))

(fn TakeDamage
  (params (newHealth :type Integer))
  (bind _output_get (Variables|Default|SetHealth (- (Variables|Default|GetHealth) newHealth)))
  (return _output_get))