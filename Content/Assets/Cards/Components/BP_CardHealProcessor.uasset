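; BP_CardHealProcessor is a card component that applies a played card's healing effects to the character who played it.
; ProcessCard loops over the card's effects and picks out each HealEffect.
; For each, it builds a GAS spec from GE_Damage, sets the heal amount through the GameplayEffect.Combat.Healing SetByCaller tag and applies it to the source's own ability system.
; It then prints the effect's text message.
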(event EventProcessCard
  (params (Card :type Card%20Object%20Reference) (SourceCharacter :type Basic%20Character%20Object%20Reference) (TargetCharacter :type Basic%20Character%20Object%20Reference))
  (bind _abilitysystemcomponent (Variables|/Script/CS3247_Project.BasicCharacter|GetAbilitySystemComponent SourceCharacter))
  (for _array_element (Variables|/Script/CS3247_Project.Card|GetEffects Card)
    (Utilities|IsValid (Class|CardEffect|GetEffect _array_element "/Script/CS3247_Project.HealEffect")
      (:Is%20Valid
        (bind _asheal_effect (Utilities|Casting|CastToHealEffect (Class|CardEffect|GetEffect _array_element "/Script/CS3247_Project.HealEffect")))
        (bind _returnvalue (Ability|GameplayEffect|AssignTagSetbyCallerMagnitude (GameplayEffects|MakeOutgoingSpec :self _abilitysystemcomponent :GameplayEffectClass "/Game/Assets/GameplayAbilities/GameplayeEffects/GE_Damage.GE_Damage_C") "(TagName=\"GameplayEffect.Combat.Healing\")" (Math|Conversions|ToFloat(Integer) (Class|HealEffect|GetHealAmount _asheal_effect))))
        (GameplayEffects|ApplyGameplayEffectSpecToTarget _abilitysystemcomponent _returnvalue _abilitysystemcomponent)
        (bind _returnvalue_2 (Class|Localisable|ToText(Message) _asheal_effect))
        (Development|PrintText 0 _returnvalue_2)))))