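; Player controller component that runs card crafting sessions at a workbench, where ingredients become linked nodes in a recipe graph.
; Workbench events set the recipe's root and connect or break node links, printing results as debug text.
; Using the recipe forges a card through the player deck subsystem and broadcasts a preview with an inventory-based affordability flag.
; Crafting broadcasts that card and starts a fresh recipe, without rechecking or deducting costs here.
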(event EventBeginPlay
  (bind _asbp_player_controller (Utilities|Casting|CastToBP_PlayerController (Components|GetOwner)))
  (bind _playerstate (Default|GetPlayerState _asbp_player_controller))
  (Variables|Default|SetPlayerState _playerstate)
  (CallFunction|EventNewSession))

(event Custom|Event%20On%20Use%20Recipe
  ;[0.15 0.15 0.15 0.5] Craft a new card and preview it
  (bind _returnvalue (Class|CardRecipe|Forge (Variables|Default|GetCurrentRecipe) (Subsystems|GetPlayerDeckSubsystem) false))
  (bind _output_get (Variables|Default|SetCraftedCard _returnvalue))
  (bind _bcanafford (Workbench|CanAffordtoCraft))
  (Default|CallOnPreviewCard _output_get _bcanafford))

(event Custom|Event%20NewSession
  ;[0.15 0.15 0.15 0.5] Start a new crafting session
  (bind _returnvalue (Game|ConstructObjectfromClass (Subsystems|GetPlayerDeckSubsystem) "/Script/CS3247_Project.CardRecipe"))
  (Variables|Default|SetCurrentRecipe _returnvalue)
  (Variables|Default|SetCraftedCard 0))

(event Custom|Event%20On%20Set%20Root%20Node
  (params (Root :type Card%20Node%20Object%20Reference))
  (Variables|/Script/CS3247_Project.CardRecipe|SetSource (Variables|Default|GetCurrentRecipe) Root))

(event Custom|Event%20On%20Invalidate%20Recipe
  (Variables|Default|SetCraftedCard 0)
  (Default|CallOnClearPreview))

(event Custom|Event%20On%20Craft%20Card
  (Default|CallOnCardCrafted (Variables|Default|GetCraftedCard))
  (Development|PrintString "New card crafted!")
  (CallFunction|EventNewSession))

(event Custom|Event%20On%20Disconnect%20Nodes
  (params (ParentNode :type Card%20Node%20Object%20Reference) (ChildNode :type Card%20Node%20Object%20Reference))
  ;[0.15 0.15 0.15 0.5] Disconnect two nodes
  (if (and (Utilities|IsValid ParentNode) (Utilities|IsValid ChildNode))
    (bind (_errormsg _returnvalue) (Class|CardNode|BreakLinkwith ParentNode ChildNode))
    (if _returnvalue
      (Development|PrintText (Utilities|Text|FormatText (Utilities|Text|MakeLiteralText "{0} -> {1} is connected") (Class|Localisable|ToText ParentNode) (Class|Localisable|ToText ChildNode)))
      (else
        (Development|PrintText _errormsg true true "(R=1.000000,G=0.000000,B=0.000000,A=1.000000)")))))

(event Custom|Event%20On%20Connect%20Nodes
  (params (ParentNode :type Card%20Node%20Object%20Reference) (ChildNode :type Card%20Node%20Object%20Reference))
  ;[0.15 0.15 0.15 0.5] Connect two nodes
  (bind _bisvalidconnection (Workbench|IsValidConnection ParentNode ChildNode))
  (if _bisvalidconnection
    (bind (_errormsg _returnvalue) (Class|CardNode|AddSuccessor ParentNode ChildNode))
    (if _returnvalue
      (bind _returnvalue_2 (Class|Localisable|ToText(Message) ParentNode))
      (bind _returnvalue_3 (Class|Localisable|ToText(Message) ChildNode))
      (Development|PrintText (Utilities|Text|FormatText (Utilities|Text|MakeLiteralText "{0} -> {1} is connected") _returnvalue_2 _returnvalue_3))
      (else
        (Development|PrintText _errormsg true true "(R=1.000000,G=0.000000,B=0.000000,A=1.000000)")))))

(fn AddIngredient
  (params (Ingredient :type Card%20Ingredient%20Object%20Reference))
  (bind _returnvalue (Class|CardIngredient|WrapIntoNode Ingredient (Subsystems|GetPlayerDeckSubsystem)))
  (return _returnvalue))

(fn IsValidConnection
  (params (Predecessor :type Card%20Node%20Object%20Reference) (Successor :type Card%20Node%20Object%20Reference))
  (Utilities|IsValid Predecessor
    (:Is%20Valid
      (Utilities|IsValid Successor
        (:Is%20Valid
          (return (!= Predecessor Successor)))
        (:Is%20Not%20Valid
          (return false))))
    (:Is%20Not%20Valid
      (return false))))

(fn CanAffordtoCraft
  (bind _currentrecipe (Variables|Default|GetCurrentRecipe))
  (bind _returnvalue (Class|CardRecipe|GetCosts _currentrecipe))
  (bind _keys (Utilities|Map|Keys _returnvalue))
  (for _array_element _keys
    (if (Class|InventoryComponent|HasEnough (Variables|/Game/Assets/Characters/Player/BP_DungeonSlayerPlayerState.BP_DungeonSlayerPlayerState_C|GetPlayerInventory (Variables|Default|GetPlayerState)) _array_element (.Value (Utilities|Map|Find _returnvalue _array_element)))
      (Development|PrintString "Hello")
      (else
        (return false))))
  (return true))