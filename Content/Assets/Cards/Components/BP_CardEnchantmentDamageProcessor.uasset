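; Card processor that deals enchantment damage from a played card's effects, from the source character to the target character.
; For each EnchantmentDamageEffect on the card, it walks the map of damage tags to amounts.
; Each entry becomes a GE_Damage spec with the key as asset tag and the value as SetByCaller magnitude, applied through GAS.
; The effect's text message is printed after every application.
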(event EventProcessCard
  (params (Card :type Card%20Object%20Reference) (SourceCharacter :type Basic%20Character%20Object%20Reference) (TargetCharacter :type Basic%20Character%20Object%20Reference))
  (bind _abilitysystemcomponent (Variables|/Script/CS3247_Project.BasicCharacter|GetAbilitySystemComponent SourceCharacter))
  (for _array_element (Variables|/Script/CS3247_Project.Card|GetEffects Card)
    (bind _asenchantment_damage_effect (Utilities|Casting|CastToEnchantmentDamageEffect (Class|CardEffect|GetEffect _array_element "/Script/CS3247_Project.EnchantmentDamageEffect")))
    (bind _keys (Utilities|Map|Keys (Variables|/Script/CS3247_Project.EnchantmentDamageEffect|GetEnchantmentDamages _asenchantment_damage_effect)))
    (for _array_element_2 _keys
      (bind _returnvalue (Ability|GameplayEffect|AddAssetTag (GameplayEffects|MakeOutgoingSpec :self _abilitysystemcomponent :GameplayEffectClass "/Game/Assets/GameplayAbilities/GameplayeEffects/GE_Damage.GE_Damage_C") _array_element_2))
      (bind _returnvalue_2 (Ability|GameplayEffect|AssignTagSetbyCallerMagnitude _returnvalue "(TagName=\"GameplayEffect.Combat.Damage\")" (.Value (Utilities|Map|Find (Variables|/Script/CS3247_Project.EnchantmentDamageEffect|GetEnchantmentDamages _asenchantment_damage_effect) _array_element_2))))
      (GameplayEffects|ApplyGameplayEffectSpecToTarget _abilitysystemcomponent _returnvalue_2 (Variables|/Script/CS3247_Project.BasicCharacter|GetAbilitySystemComponent TargetCharacter))
      (bind _returnvalue_3 (Class|Localisable|ToText(Message) _asenchantment_damage_effect))
      (Development|PrintText 0 _returnvalue_3))))