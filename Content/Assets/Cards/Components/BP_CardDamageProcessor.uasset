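; Card component that applies the damage effects of a card from a source character to a target character through the Gameplay Ability System.
; ProcessCard loops over the card's effects and, for each damage effect, builds a GE_Damage spec from the source, tagged with the damage type.
; The damage value is passed as a SetByCaller magnitude, then the spec is applied to the target and the effect's text message is printed.
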(event EventProcessCard
  (params (Card :type Card%20Object%20Reference) (SourceCharacter :type Basic%20Character%20Object%20Reference) (TargetCharacter :type Basic%20Character%20Object%20Reference))
  (bind _abilitysystemcomponent (Variables|/Script/CS3247_Project.BasicCharacter|GetAbilitySystemComponent SourceCharacter))
  (for _array_element (Variables|/Script/CS3247_Project.Card|GetEffects Card)
    (Utilities|IsValid (Class|CardEffect|GetEffect _array_element "/Script/CS3247_Project.DamageEffect")
      (:Is%20Valid
        (bind _asdamage_effect (Utilities|Casting|CastToDamageEffect (Class|CardEffect|GetEffect _array_element "/Script/CS3247_Project.DamageEffect")))
        (bind _returnvalue (Ability|GameplayEffect|AddAssetTag (GameplayEffects|MakeOutgoingSpec :self _abilitysystemcomponent :GameplayEffectClass "/Game/Assets/GameplayAbilities/GameplayeEffects/GE_Damage.GE_Damage_C") (Variables|/Script/CS3247_Project.DamageEffect|GetDamageType _asdamage_effect)))
        (bind _returnvalue_2 (Ability|GameplayEffect|AssignTagSetbyCallerMagnitude _returnvalue "(TagName=\"GameplayEffect.Combat.Damage\")" (Math|Conversions|ToFloat(Integer) (Class|DamageEffect|GetDamageValue _asdamage_effect))))
        (GameplayEffects|ApplyGameplayEffectSpecToTarget _abilitysystemcomponent _returnvalue_2 (Variables|/Script/CS3247_Project.BasicCharacter|GetAbilitySystemComponent TargetCharacter))
        (bind _returnvalue_3 (Class|Localisable|ToText(Message) _asdamage_effect))
        (Development|PrintText 0 _returnvalue_3)))))