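; BP_CardDefenceProcessor is a card component meant to process the defence effects of a card.
; Its ProcessCard event loops through the card's effects and checks each for a DefenceEffect, but takes no action on a match.
; A disconnected chain would apply GE_Defend from the source character to itself through GAS, passing GetHealAmount as a set-by-caller magnitude under the Healing tag, then print a message.
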(event EventProcessCard
  (params (Card :type Card%20Object%20Reference) (SourceCharacter :type Basic%20Character%20Object%20Reference) (TargetCharacter :type Basic%20Character%20Object%20Reference))
  (for _array_element (Variables|/Script/CS3247_Project.Card|GetEffects Card)
    (Utilities|IsValid (Class|CardEffect|GetEffect _array_element "/Script/CS3247_Project.DefenceEffect"))))