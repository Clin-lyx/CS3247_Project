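; Actor component on the player controller that executes played cards against a target character.
; On BeginPlay it caches the controlled player character and builds an ordered list of processor objects for mana cost, damage, heal, enchantment damage and defence.
; OnExecuteCard passes the card, player character and target through every processor in turn, so each card effect type lives in its own processor class.
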(event Custom|Event%20On%20Execute%20Card
  (params (CardData :type Card%20Object%20Reference) (TargetCharacter :type Basic%20Character%20Object%20Reference))
  (for _array_element (Variables|Default|GetProcessors)
    (Class|CardProcessor|ProcessCard _array_element CardData (Variables|Default|GetPlayerCharacter) TargetCharacter)))

(event EventBeginPlay
  (bind _asbp_player_controller (Utilities|Casting|CastToBP_PlayerController (Components|GetOwner)))
  (bind _asbp_player_character (Utilities|Casting|CastToBP_PlayerCharacter (Pawn|GetControlledPawn _asbp_player_controller)))
  (Variables|Default|SetPlayerCharacter _asbp_player_character)
  (bind _returnvalue (Game|ConstructObjectfromClass "/Game/Assets/Cards/Components/BP_CardManaCostProcessor.BP_CardManaCostProcessor_C"))
  (Utilities|Array|Add (Variables|Default|GetProcessors) _returnvalue)
  (bind _returnvalue_2 (Game|ConstructObjectfromClass "/Game/Assets/Cards/Components/BP_CardDamageProcessor.BP_CardDamageProcessor_C"))
  (Utilities|Array|Add (Variables|Default|GetProcessors) _returnvalue_2)
  (bind _returnvalue_3 (Game|ConstructObjectfromClass "/Game/Assets/Cards/Components/BP_CardHealProcessor.BP_CardHealProcessor_C"))
  (Utilities|Array|Add (Variables|Default|GetProcessors) _returnvalue_3)
  (bind _returnvalue_4 (Game|ConstructObjectfromClass "/Game/Assets/Cards/Components/BP_CardEnchantmentDamageProcessor.BP_CardEnchantmentDamageProcessor_C"))
  (Utilities|Array|Add (Variables|Default|GetProcessors) _returnvalue_4)
  (bind _returnvalue_5 (Game|ConstructObjectfromClass "/Game/Assets/Cards/Components/BP_CardDefenceProcessor.BP_CardDefenceProcessor_C"))
  (Utilities|Array|Add (Variables|Default|GetProcessors) _returnvalue_5))