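; BP_EncounterZone is a trigger zone that starts a combat encounter with a random enemy formation when the player enters it.
; BeginPlay totals the weights in DT_EnemyFormations, and SelectEnemies makes a cumulative-weight random pick from that table.
; The chosen enemies spawn evenly spaced between two anchor components.
; The player's view turns toward their midpoint, and a spawned BP_TurnManager receives them to begin combat.
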(event OnComponentBeginOverlap(TriggerZone)
  (params (OverlappedComponent :type Primitive%20Component%20Object%20Reference) (OtherActor :type Actor%20Object%20Reference) (OtherComp :type Primitive%20Component%20Object%20Reference) (OtherBodyIndex :type Integer) (bFromSweep :type Boolean) (SweepResult :type Hit%20Result%20Structure%20%28by%20ref%29))
  ;[0.15 0.15 0.15 0.5] Spawn Enemies and TurnManager
  (bind _asbp_player_character (Utilities|Casting|CastToBP_PlayerCharacter OtherActor))
  (bind _output_get (Variables|Default|SetPlayerCharacter _asbp_player_character))
  (bind _enemies_to_spawn (CallFunction|SelectEnemies))
  (bind (_enemycharacters _lookatrotation) (CallFunction|SpawnEnemies _enemies_to_spawn))
  (Pawn|SetControlRotation (Pawn|GetController _output_get) _lookatrotation)
  (bind _returnvalue (Game|SpawnActorfromClass "/Game/Assets/Combat/BP_TurnManager.BP_TurnManager_C" (Transformation|GetActorTransform self) "Undefined" "MultiplyWithRoot" 0 _output_get 0))
  (Default|EventonCombatStart _returnvalue _enemycharacters))

(event EventBeginPlay
  (bind _outrownames (DataTable|GetDataTableRowNames "/Game/Assets/Characters/Enemies/Data/DT_EnemyFormations.DT_EnemyFormations"))
  (for _array_element _outrownames
    (bind _returnvalue (Utilities|GetDataTableRow "/Game/Assets/Characters/Enemies/Data/DT_EnemyFormations.DT_EnemyFormations" _array_element)
      (:then
        (Variables|EnemySpawning|SetTotalWeight (+ (.Weight (Utilities|Struct|BreakS_EnemyFormationRowStructure _returnvalue)) (Variables|EnemySpawning|GetTotalWeight)))))))

(fn ConstructionScript)

(fn SelectEnemies
  (LocalVariables|SetIndex (Math|Random|RandomIntegerinRange 1 (Variables|EnemySpawning|GetTotalWeight)))
  (bind _outrownames (DataTable|GetDataTableRowNames "/Game/Assets/Characters/Enemies/Data/DT_EnemyFormations.DT_EnemyFormations"))
  (for _array_element _outrownames
    (bind _returnvalue (Utilities|GetDataTableRow "/Game/Assets/Characters/Enemies/Data/DT_EnemyFormations.DT_EnemyFormations" _array_element)
      (:then
        (bind _output_get (LocalVariables|SetCumulativeWeight (+ (.Weight (Utilities|Struct|BreakS_EnemyFormationRowStructure _returnvalue)) (LocalVariables|GetCumulativeWeight))))
        (if (>= _output_get (LocalVariables|GetIndex))
          (return (.Enemies (Utilities|Struct|BreakS_EnemyFormationRowStructure _returnvalue))))))))

(fn FindSpawnTransform
  (params (NumberOfEnemies :type Integer) (CurrentEnemyIndex :type Integer))
  (bind _anker1 (Variables|Default|GetAnker1))
  (bind _returnvalue (Transformation|GetWorldLocation _anker1))
  (return (Math|Conversions|ToTransform(Vector) (+ (* (+ CurrentEnemyIndex 1) (/ (- (Transformation|GetWorldLocation (Variables|Default|GetAnker2)) _returnvalue) (+ NumberOfEnemies 1))) _returnvalue))))

(fn SpawnEnemies
  (params (EnemyData :type Array%20of%20Enemy%20Object%20References))
  (bind _spawnedenemies (LocalVariables|GetSpawnedEnemies))
  (for (_array_element _array_index) EnemyData
    (bind _spawn_transform (CallFunction|FindSpawnTransform (Utilities|Array|Length EnemyData) _array_index))
    (bind _returnvalue (Game|SpawnActorfromClass "/Game/Assets/Characters/Enemies/BP_EnemyCharacter.BP_EnemyCharacter_C" _spawn_transform "Undefined" "MultiplyWithRoot" 0 _array_element 0))
    (Utilities|Array|Add (LocalVariables|GetSpawnedEnemies) _returnvalue))
  (return (LocalVariables|GetSpawnedEnemies) (Math|Rotator|FindLookatRotation (Camera|GetCameraLocation (Game|GetPlayerCameraManager 0)) (/ (+ (Transformation|GetActorLocation (Utilities|Array|Get(acopy) _spawnedenemies)) (Transformation|GetActorLocation (Utilities|Array|Get(acopy) (LocalVariables|GetSpawnedEnemies) (Utilities|Array|LastIndex _spawnedenemies)))) 2))))