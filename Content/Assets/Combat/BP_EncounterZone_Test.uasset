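; Test encounter zone that starts combat when the player overlaps its trigger, then destroys itself.
; It turns the player toward an anchor, spawns tank enemies evenly between two player-relative anchor points, and aims the control rotation at their midpoint.
; It then spawns BP_CombatMediator with the player and enemies.
; A weighted random pick from DT_EnemyFormations is defined but never called; spawning uses fixed tank data.
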(event OnComponentBeginOverlap(TriggerZone)
  (params (OverlappedComponent :type Primitive%20Component%20Object%20Reference) (OtherActor :type Actor%20Object%20Reference) (OtherComp :type Primitive%20Component%20Object%20Reference) (OtherBodyIndex :type Integer) (bFromSweep :type Boolean) (SweepResult :type Hit%20Result%20Structure%20%28by%20ref%29))
  ;[0.15 0.15 0.15 0.5] Spawn Enemies and TurnManager
  (bind _asbp_player_character (Utilities|Casting|CastToBP_PlayerCharacter OtherActor))
  (bind _output_get (Variables|Default|SetPlayerCharacter _asbp_player_character))
  (CallFunction|AdjustPlayerCameraFacing _output_get)
  (bind (_enemycharacters _lookatrotation) (CallFunction|SpawnEnemies))
  (Pawn|SetControlRotation (Pawn|GetController _output_get) _lookatrotation)
  (Game|SpawnActorfromClass "/Game/Assets/Combat/BP_CombatMediator.BP_CombatMediator_C" (Transformation|GetActorTransform self) "AlwaysSpawn" "MultiplyWithRoot" 0 _output_get _enemycharacters 0)
  (Actor|DestroyActor))

(event Custom|Adjust%20Player%20Camera%20Facing
  (params (Player%20Character :type BP%20Player%20Character%20Object%20Reference))
  (bind _returnvalue (Transformation|GetActorRotation Player%20Character))
  (bind (_roll _pitch) (Math|Rotator|BreakRotator _returnvalue))
  (Variables|Default|SetStaterRotation _returnvalue)
  (bind _output_get (Variables|Default|SetTargetRotation (Math|Rotator|MakeRotator _roll _pitch (.Yaw (Math|Rotator|BreakRotator (Math|Rotator|FindLookatRotation (Transformation|GetActorLocation Player%20Character) (Transformation|GetWorldLocation (Variables|Default|GetAnker))))))))
  (Transformation|SetActorRotation Player%20Character _output_get))

(fn ConstructionScript)

(fn SelectEnemies
  (LocalVariables|SetIndex (Math|Random|RandomIntegerinRange 1 (Variables|EnemySpawning|GetTotalWeight)))
  (bind _outrownames (DataTable|GetDataTableRowNames "/Game/Assets/Characters/Enemies/Data/DT_EnemyFormations.DT_EnemyFormations"))
  (for _array_element _outrownames
    (bind _returnvalue (Utilities|GetDataTableRow "/Game/Assets/Characters/Enemies/Data/DT_EnemyFormations.DT_EnemyFormations" _array_element)
      (:then
        (bind _output_get (LocalVariables|SetCumulativeWeight (+ (.Weight (Utilities|Struct|BreakS_EnemyFormationRowStructure _returnvalue)) (LocalVariables|GetCumulativeWeight))))
        (if (>= _output_get (LocalVariables|GetIndex))
          (return (.Enemies (Utilities|Struct|BreakS_EnemyFormationRowStructure _returnvalue))))))))

(fn FindSpawnTransform
  (params (NumberOfEnemies :type Integer) (CurrentEnemyIndex :type Integer) (Anker1Loc :type Vector) (Anker2Loc :type Vector))
  (return (Math|Conversions|ToTransform(Vector) (+ (* (+ CurrentEnemyIndex 1) (/ (- Anker1Loc Anker2Loc) (+ (Variables|Default|GetEnemyNumber) 1))) Anker2Loc))))

(fn SpawnEnemies
  (bind _spawnedenemies (LocalVariables|GetSpawnedEnemies))
  (bind _result (Math|Integer|DecrementInt (Variables|Default|GetEnemyNumber))
    (:%20%20
      (for _index (range 0 _result)
        (bind (_anchor1 _anchor2) (CallFunction|FindTwoAnkers))
        (bind _spawn_transform (CallFunction|FindSpawnTransform 0 _index _anchor1 _anchor2))
        (bind _returnvalue (Game|SpawnActorfromClass "/Game/Assets/Characters/Enemies/BP_Tank.BP_Tank_C" _spawn_transform "Undefined" "MultiplyWithRoot" 0 "/Game/Assets/Characters/Enemies/Data/DA_EnemyTank.DA_EnemyTank" 0))
        (Utilities|Array|Add (LocalVariables|GetSpawnedEnemies) _returnvalue)
        (Transformation|SetActorRotation _returnvalue (Math|Rotator|FindLookatRotation (Transformation|GetActorLocation (Variables|Default|GetPlayerCharacter)) (Transformation|GetActorLocation _returnvalue))))
      (return (LocalVariables|GetSpawnedEnemies) (Math|Rotator|FindLookatRotation (Camera|GetCameraLocation (Game|GetPlayerCameraManager 0)) (/ (+ (Transformation|GetActorLocation (Utilities|Array|Get(acopy) (LocalVariables|GetSpawnedEnemies))) (Transformation|GetActorLocation (Utilities|Array|Get(acopy) _spawnedenemies (Utilities|Array|LastIndex _spawnedenemies)))) 2))))))

(fn FindTwoAnkers
  (bind _returnvalue (Class|GenerateEnemySpawnAnchors|GenerateAnchorsBasedonPlayer (Variables|Default|GetPlayerCharacter) 5e+02 4e+02))
  (return (Utilities|Array|Get(acopy) _returnvalue) (Utilities|Array|Get(acopy) _returnvalue 1)))