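; BP_Pot is a map interactable pot that holds a weighted pool of game item rewards, such as spells and card enchantments.
; On BeginPlay it fills its RandomSelectorComponent with item data assets and their weights.
; Its RandomSelect function returns a weighted pick from that component, while the activation and deactivation events are left empty.
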(event Custom|Event%20On%20Activated)

(event Custom|Event%20On%20Deactivated)

(event EventBeginPlay
  (bind _randomselectorcomponent (Variables|Default|GetRandomSelectorComponent))
  (Utilities|FlowControl|Sequence
    (:then_0
      (Default|Add _randomselectorcomponent "/Game/Assets/Cards/Crafting/Ingredients/FlowControl/DA_DualCasting.DA_DualCasting" 1.0))
    (:then_1
      (Default|Add _randomselectorcomponent "/Game/Assets/Cards/Crafting/Ingredients/Enchantments/DA_CardEnchantmentPowerUp.DA_CardEnchantmentPowerUp" 2.0))
    (:then_2
      (Default|Add _randomselectorcomponent "/Game/Assets/Cards/Crafting/Ingredients/Impacts/DA_FireSparks.DA_FireSparks" 1.0))
    (:then_3
      (Default|Add _randomselectorcomponent "/Game/Assets/Cards/Crafting/Ingredients/Impacts/DA_HealerHand.DA_HealerHand" 0.7))
    (:then_4
      (Default|Add _randomselectorcomponent "/Game/Assets/Cards/Crafting/Ingredients/Enchantments/DA_CardEnchantmentScorch.DA_CardEnchantmentScorch" 0.3))))

(event Collision|EventActorBeginOverlap
  (params (OtherActor :type Actor%20Object%20Reference)))

(event EventTick
  (params (DeltaSeconds :type Float%20%28single-precision%29)))

(fn ConstructionScript)

(fn RandomSelect
  (bind _selected (Default|RandomSelect (Variables|Default|GetRandomSelectorComponent)))
  (return _selected))