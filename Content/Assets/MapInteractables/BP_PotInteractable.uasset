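; BP_PotInteractable is a lootable pot interactable that gives random items to the player who interacts with it.
; On Interact, it draws PollTimes items from its BP_Pot child actor, tallies them in RewardMap, and opens the player's loot container.
; The items go straight to the PlayerState and the pot is marked Opened.
; An opened pot skips the parent in-range logic and closes the container when the player leaves.
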(event Custom|Event%20OnPlayerOutOfRange
  (params (Player :type Player%20Character%20Object%20Reference))
  (if (not (Variables|Default|GetReEntering))
    (if (Variables|Default|GetOpened)
      (Default|CallOnCloseLootContainer (Variables|Default|GetPlayerInRange))
      (Variables|Default|SetReEntering true))
    (|CallParentFunction Player)))

(event EventBeginPlay
  (bind _asbp_pot (Utilities|Casting|CastToBP_Pot (Variables|/Script/Engine.ChildActorComponent|GetChildActor (Variables|Default|GetInteractableActor))))
  (Variables|Default|SetPot _asbp_pot))

(event EventOnPlayerinRange
  (params (Player :type Player%20Character%20Object%20Reference))
  (Development|PrintString (Utilities|String|ToString(Boolean) (Variables|Default|GetOpened)))
  (if (not (Variables|Default|GetOpened))
    (|CallParentFunction Player)))

(event Input|ActionEvents|InputActionInteract
  (params (Key :type Key%20Structure :default "None"))
  (bind _rewardmap (Variables|Default|GetRewardMap))
  (bind _rewardmap_2 (Variables|Default|GetRewardMap))
  (:Pressed
    (while (> (Variables|Default|GetPollTimes) 0)
      (bind _gameitem (Default|RandomSelect (Variables|Default|GetPot)))
      (if (.ReturnValue (Utilities|Map|Find _rewardmap _gameitem))
        (Utilities|Map|Add _rewardmap _gameitem (+ (.Value (Utilities|Map|Find _rewardmap _gameitem)) 1))
        (else
          (Utilities|Map|Add _rewardmap _gameitem 1)))
      (Variables|Default|SetPollTimes (- (Variables|Default|GetPollTimes) 1)))
    (Default|CallOnOpenLootContainer (Variables|Default|GetPlayerInRange) (Variables|Default|GetRewardMap))
    (bind _playerstate (Default|GetPlayerState (Variables|Default|GetPlayerInRange)))
    (bind _keys (Utilities|Map|Keys _rewardmap_2))
    (for _array_element _keys
      (Default|EventonCollectItems _playerstate _array_element (.Value (Utilities|Map|Find _rewardmap_2 _array_element)))
      (Variables|Default|SetOpened true))))

(fn ConstructionScript
  (|CallParentFunction))