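; Candle prop for the enchanting station that can be lit and put out.
; The point light starts hidden at BeginPlay.
; OnLit activates the flame particle and shows the light, and OnPutoff deactivates the particle and hides the light.
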(event Custom|Event%20On%20Lit
  (Components|Activation|Activate (Variables|Default|GetFlameParticle) true)
  (Rendering|SetVisibility (Variables|Default|GetPointLight) true false))

(event Custom|Event%20On%20Put%20off
  (Components|Activation|Deactivate (Variables|Default|GetFlameParticle))
  (Rendering|SetVisibility (Variables|Default|GetPointLight) false false))

(event EventBeginPlay
  (Rendering|SetVisibility (Variables|Default|GetPointLight) false false))

(fn ConstructionScript)