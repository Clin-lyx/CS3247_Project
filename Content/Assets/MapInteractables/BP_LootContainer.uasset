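; BP_LootContainer is a map interactable that rolls random loot and grants it to the player who interacts with it.
; On BeginPlay it builds a weighted selector from PossibleLoots, polls it a random number of times and totals the results in Loots.
; Range events show or close the loot display through PlayerInRange and call empty OnOpen/OnClose hooks.
; Interact sends all items to the PlayerState, removes the collision box and optionally destroys the actor.
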(event EventBeginPlay
  (bind _keys (Utilities|Map|Keys (Variables|Default|GetPossibleLoots)))
  (for _array_element _keys
    (Default|Add (Variables|Default|GetSelector) _array_element (Math|Conversions|ToFloat(Integer) (.Value (Utilities|Map|Find (Variables|Default|GetPossibleLoots) _array_element)))))
  (for _index (range 1 (Math|Random|RandomIntegerinRange 1 (Variables|Default|GetMaxPollTimes)))
    (Development|PrintText (Utilities|Text|FormatText "{0} polls {1}" self _index))
    (bind _selected (Default|RandomSelect (Variables|Default|GetSelector)))
    (if (.ReturnValue (Utilities|Map|Find (Variables|Default|GetLoots) (.Item (Utilities|Struct|BreakS_Loot _selected))))
      (Utilities|Map|Add (Variables|Default|GetLoots) (.Item (Utilities|Struct|BreakS_Loot _selected)) (+ (.Value (Utilities|Map|Find (Variables|Default|GetLoots) (.Item (Utilities|Struct|BreakS_Loot _selected)))) (.Qty (Utilities|Struct|BreakS_Loot _selected))))
      (else
        (Utilities|Map|Add (Variables|Default|GetLoots) (.Item (Utilities|Struct|BreakS_Loot _selected)) (.Qty (Utilities|Struct|BreakS_Loot _selected)))))))

(event EventOnPlayerinRange
  (params (Player :type Player%20Character%20Object%20Reference))
  (CallFunction|OnOpen)
  (|CallParentFunction Player)
  (Default|CallOnCloseLootContainer (Variables|Default|GetPlayerInRange))
  (Default|CallOnOpenLootContainer (Variables|Default|GetPlayerInRange) (Variables|Default|GetLoots)))

(event EventOnPlayerOutOfRange
  (params (Player :type Player%20Character%20Object%20Reference))
  (CallFunction|OnClose)
  (Default|CallOnCloseLootContainer (Variables|Default|GetPlayerInRange))
  (|CallParentFunction Player))

(event Input|ActionEvents|InputActionInteract
  (params (Key :type Key%20Structure :default "None"))
  (bind _loots (Variables|Default|GetLoots))
  (:Pressed
    (bind _playerstate (Default|GetPlayerState (Variables|Default|GetPlayerInRange)))
    (bind _keys (Utilities|Map|Keys _loots))
    (for _array_element _keys
      (Default|EventonCollectItems _playerstate _array_element (.Value (Utilities|Map|Find _loots _array_element))))
    (Components|DestroyComponent (Variables|Default|GetCollisionBox))
    (bind _asbp_player_character (Utilities|Casting|CastToBP_PlayerCharacter (Pawn|GetControlledPawn (Variables|Default|GetPlayerInRange))))
    (Class|InteractableObject|OnPlayerOutOfRange _asbp_player_character)
    (if (Variables|Default|GetbDestroyOnInteract)
      (Actor|DestroyActor))))

(fn ConstructionScript)

(fn OnOpen)

(fn OnClose)