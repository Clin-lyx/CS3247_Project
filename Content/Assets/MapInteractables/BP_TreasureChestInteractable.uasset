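; Treasure chest map interactable that gives the player in range a randomized set of rewards.
; It wraps a BP_TreasureChest child actor, cached on BeginPlay, and activates or deactivates it as a player enters or leaves range.
; On Interact, it polls the chest's RandomSelect until PollTimes runs out, tallying duplicates in RewardMap.
; It then passes the map to the player's open-loot-container call.
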(event EventBeginPlay
  (bind _asbp_treasure_chest (Utilities|Casting|CastToBP_TreasureChest (Variables|/Script/Engine.ChildActorComponent|GetChildActor (Variables|Default|GetInteractableActor))))
  (Variables|Default|SetTreasureChest _asbp_treasure_chest))

(event EventOnPlayerinRange
  (params (Player :type Player%20Character%20Object%20Reference))
  (|CallParentFunction Player)
  (Default|EventonActivated (Variables|Default|GetTreasureChest)))

(event EventOnPlayerOutOfRange
  (params (Player :type Player%20Character%20Object%20Reference))
  (|CallParentFunction Player)
  (Default|EventonDeactivated (Variables|Default|GetTreasureChest)))

(event Input|ActionEvents|InputActionInteract
  (params (Key :type Key%20Structure :default "None"))
  (bind _rewardmap (Variables|Default|GetRewardMap))
  (:Pressed
    (while (> (Variables|Default|GetPollTimes) 0)
      (bind _gameitem (Default|RandomSelect (Variables|Default|GetTreasureChest)))
      (if (.ReturnValue (Utilities|Map|Find _rewardmap _gameitem))
        (Utilities|Map|Add _rewardmap _gameitem (+ (.Value (Utilities|Map|Find _rewardmap _gameitem)) 1))
        (else
          (Utilities|Map|Add _rewardmap _gameitem 1)))
      (Variables|Default|SetPollTimes (- (Variables|Default|GetPollTimes) 1)))
    (Default|CallOnOpenLootContainer (Variables|Default|GetPlayerInRange) (Variables|Default|GetRewardMap))))

(fn ConstructionScript
  (|CallParentFunction))