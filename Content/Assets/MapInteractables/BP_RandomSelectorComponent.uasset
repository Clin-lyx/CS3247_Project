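; Component for weighted random selection of loot, holding a map of loot entries to weights.
; Add and Remove edit the map.
; RandomSelect sums the weights, then walks the normalized cumulative ranges and returns the key whose range contains a random float.
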(event EventBeginPlay)

(event EventTick
  (params (DeltaSeconds :type Float%20%28single-precision%29)))

(fn Add
  (params (Loot :type S%20Loot%20Structure) (Weight :type Float%20%28double-precision%29))
  (Utilities|Map|Add (Variables|Default|GetWeightedMap) Loot Weight))

(fn Remove
  (params (Loot :type S%20Loot%20Structure))
  (Utilities|Map|Remove (Variables|Default|GetWeightedMap) Loot))

(fn RandomSelect
  (bind _weightedmap (Variables|Default|GetWeightedMap))
  (Utilities|FlowControl|Sequence
    (:then_0
      (LocalVariables|SetSelector (Math|Random|RandomFloat)))
    (:then_1
      (bind _values (Utilities|Map|Values _weightedmap))
      (for _array_element _values
        (LocalVariables|SetTotal (+ (LocalVariables|GetTotal) _array_element))))
    (:then_2
      (for (_array_element_2 _array_index) _values
        (LocalVariables|SetLastCumulative (LocalVariables|GetCumulative))
        (LocalVariables|SetCumulative (+ (/ _array_element_2 (LocalVariables|GetTotal)) (LocalVariables|GetCumulative)))
        (if (and (> (LocalVariables|GetSelector) (LocalVariables|GetLastCumulative)) (>= (LocalVariables|GetCumulative) (LocalVariables|GetSelector)))
          (bind _keys (Utilities|Map|Keys _weightedmap))
          (return (Utilities|Array|Get(acopy) _keys _array_index)))))))