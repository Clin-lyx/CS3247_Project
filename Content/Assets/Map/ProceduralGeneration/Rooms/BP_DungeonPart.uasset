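; BP_DungeonPart is a room piece for procedural dungeon generation, exposing its exits and an overlap check on its Box.
; On BeginPlay it caches the children of SpawnPoints as possible spawn locations and hides the exit components.
; OnSpawnMapObjects shuffles the spawnable classes and cached points, then pairs them by index to spawn a random number of objects, possibly none.
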(event Custom|Event%20On%20Spawn%20Map%20Objects
  (bind _spawnpoints (Variables|Default|GetSpawnPoints))
  (bind _returnvalue (Class|SceneComponent|GetNumChildrenComponents _spawnpoints))
  (bind _returnvalue_2 (Math|Random|RandomIntegerinRange 0 _returnvalue))
  (if (> _returnvalue_2 0)
    (Utilities|Array|Shuffle (Variables|Default|GetSpawnableObjects))
    (Utilities|Array|Shuffle (Variables|Default|GetPossibleSpawnPoints))
    (for _index (range 0 (- _returnvalue_2 1))
      (Game|SpawnActorfromClass (Utilities|Array|Get(acopy) (Variables|Default|GetSpawnableObjects) _index) (Transformation|GetWorldTransform (Utilities|Array|Get(acopy) (Variables|Default|GetPossibleSpawnPoints) _index)) "AlwaysSpawn" "MultiplyWithRoot" 0 0))))

(event EventBeginPlay
  (for _array_element (Components|GetChildrenComponents (Variables|Default|GetSpawnPoints) false)
    (Utilities|Array|AddUnique (Variables|Default|GetPossibleSpawnPoints) _array_element))
  (for _array_element_2 (Components|GetChildrenComponents (Variables|Default|GetExits) false)
    (Rendering|SetVisibility _array_element_2 false true)))

(fn ConstructionScript)

(fn IsColliding
  (return (Utilities|Array|IsNotEmpty (Class|PrimitiveComponent|GetOverlappingComponents (Variables|Default|GetBox)))))

(fn FetchAllExits
  (return (Components|GetChildrenComponents (Variables|Default|GetExits) false)))