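; BP_Room_1 is a procedural dungeon room that may contain an enchanting station.
; On BeginPlay it runs the parent logic, then on a coin flip spawns a BP_EnchantingStationInteractable.
; The location comes from a random child component of EnchantingTableSpawnPointFolder, so candidate spots are defined by components placed under that folder.
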(event EventBeginPlay
  (|CallParentFunction)
  (if (Math|Random|RandomBool)
    (Game|SpawnActorfromClass "/Game/Assets/Cards/Crafting/BP_EnchantingStationInteractable.BP_EnchantingStationInteractable_C" (Math|Transform|MakeTransform (Transformation|GetWorldLocation (.OutItem (Utilities|Array|Random (Components|GetChildrenComponents (Variables|Default|GetEnchantingTableSpawnPointFolder) false)))) "0, 0, 0" "1.000000,1.000000,1.000000") "Undefined" "MultiplyWithRoot" 0 0)))

(event Collision|EventActorBeginOverlap
  (params (OtherActor :type Actor%20Object%20Reference))
  (|CallParentFunction OtherActor) ; This node is disabled and will not be called.\nDrag off pins to build functionality.
)

(event EventTick
  (params (DeltaSeconds :type Float%20%28single-precision%29))
  (|CallParentFunction DeltaSeconds) ; This node is disabled and will not be called.\nDrag off pins to build functionality.
)

(fn ConstructionScript
  (|CallParentFunction))