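; Player controller for the card-based Dungeon Slayer game, linking card crafting and card play to its components.
; On BeginPlay it checks for a Dungeon Slayer player state, then binds an event to the card crafter component's OnCardCrafted.
; OnPlayCard forwards the card to the card executor component without passing on the target character.
; A helper function returns the player state cast to the Dungeon Slayer type.
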(event Custom|Event%20On%20Play%20Card
  (params (TargetCharacter :type Basic%20Character%20Object%20Reference) (Card :type Card%20Object%20Reference))
  (Default|EventonExecuteCard (Variables|Default|GetCardExecutorComponent) Card))

(event EventBeginPlay
  (bind _asbp_dungeon_slayer_player_state (Utilities|Casting|CastToBP_DungeonSlayerPlayerState (Variables|GetPlayerState)))
  (EventDispatchers|BindEventtoOnCardCrafted (Variables|Default|GetCardCrafterComponent) (EventDispatchers|CreateEvent (Variables|/Game/Assets/Characters/Player/BP_DungeonSlayerPlayerState.BP_DungeonSlayerPlayerState_C|GetPlayerDeck _asbp_dungeon_slayer_player_state) :!event EventAddCard)))

(fn ConstructionScript)

(fn GetPlayerState
  (bind _asbp_dungeon_slayer_player_state (Utilities|Casting|CastToBP_DungeonSlayerPlayerState (Variables|GetPlayerState)))
  (return _asbp_dungeon_slayer_player_state))