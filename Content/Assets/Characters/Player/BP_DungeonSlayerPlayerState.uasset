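; Player state Blueprint for the dungeon slayer player, owning the player's inventory and card deck.
; On BeginPlay it seeds the inventory from the starting items and quantities in InitialPlayerState.
; It also forges each starting deck entry as a default card, adds it to PlayerDeck and prints a debug string.
; A collect-items event forwards picked-up items and quantities to the inventory.
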(event Custom|Event%20on%20Collect%20Items
  (params (Item :type Game%20Item%20Object%20Reference) (Qty :type Integer))
  (Default|EventonAddItem (Variables|Default|GetPlayerInventory) Item Qty))

(event EventBeginPlay
  (bind _initialplayerstate (Variables|Default|GetInitialPlayerState))
  (bind _startinginventory (Variables|/Script/CS3247_Project.StartingPlayerState|GetStartingInventory _initialplayerstate))
  (bind _keys (Utilities|Map|Keys _startinginventory))
  (for _array_element _keys
    (Default|EventonAddItem (Variables|Default|GetPlayerInventory) _array_element (.Value (Utilities|Map|Find _startinginventory _array_element))))
  (for _array_element_2 (Variables|/Script/CS3247_Project.StartingPlayerState|GetStartingDeck (Variables|Default|GetInitialPlayerState))
    (bind _returnvalue (Class|CardRecipe|Forge _array_element_2 (Variables|Default|GetPlayerDeck) true))
    (Class|DeckComponent|AddCard (Variables|Default|GetPlayerDeck) _returnvalue)
    (Development|PrintString "Hello")))

(fn ConstructionScript)