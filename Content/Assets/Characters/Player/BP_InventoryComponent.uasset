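; Player inventory component that holds ten item slots, toggles the inventory widget with I and picks up items with E.
; Pickup sphere-traces around the player's feet for a BP_ParentInventoryItems actor, with debug drawing on.
; The item goes into the first slot that is either empty or a same-name stack staying within 99.
; The widget then reloads from the component and the actor is destroyed, even if no slot accepted it.
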(event EventBeginPlay
  (bind _returnvalue (UserInterface|CreateWidget "/Game/Assets/Collectibles/WBP_Inventory.WBP_Inventory_C"))
  (Variables|Default|SetinventoryWidget _returnvalue)
  (Utilities|Array|Resize (Variables|Default|GetitemDatas) 10)
  (Default|LoadInventory (Variables|Default|GetinventoryWidget) self))

(event EventTick
  (params (DeltaSeconds :type Float%20%28single-precision%29)))

(event Input|KeyboardEvents|I
  (params (Key :type Key%20Structure :default "None"))
  (bind _inventorywidget (Variables|Default|GetinventoryWidget))
  (:Pressed
    (if (Widget|IsVisible (Variables|Default|GetinventoryWidget))
      (Widget|RemovefromParent _inventorywidget)
      (else
        (UserInterface|Viewport|AddtoViewport _inventorywidget 0)))))

(event Input|KeyboardEvents|E
  (params (Key :type Key%20Structure :default "None"))
  (bind _returnvalue (Game|GetPlayerCharacter 0))
  (bind _returnvalue_2 (Transformation|GetActorLocation _returnvalue))
  (bind _returnvalue_3 (- _returnvalue_2 "0.000000,0.000000,65.000000"))
  (:Pressed
    (bind _outhit (Collision|SphereTraceByChannel _returnvalue_3 _returnvalue_3 1.2e+02 "TraceTypeQuery1" false 0 "ForDuration"))
    (bind _asbp_parent_inventory_items (Utilities|Casting|CastToBP_ParentInventoryItems (.HitActor (Collision|BreakHitResult _outhit)))
      (:then
        (bind (_array_element _array_index) (Utilities|Array|ForEachLoopwithBreak (Variables|Default|GetitemDatas) :!label _label)
          (:LoopBody
            (if (and (== (.name (Utilities|Struct|BreakS_ItemData _array_element)) (.name (Utilities|Struct|BreakS_ItemData (Variables|/Game/Assets/Collectibles/BP_ParentInventoryItems.BP_ParentInventoryItems_C|Getitem _asbp_parent_inventory_items)))) (<= (+ (.value (Utilities|Struct|BreakS_ItemData _array_element)) (.value (Utilities|Struct|BreakS_ItemData (Variables|/Game/Assets/Collectibles/BP_ParentInventoryItems.BP_ParentInventoryItems_C|Getitem _asbp_parent_inventory_items)))) 99))
              (Utilities|Array|SetArrayElem (Variables|Default|GetitemDatas) _array_index (Utilities|Struct|MakeS_ItemData (.name (Utilities|Struct|BreakS_ItemData _array_element)) (+ (.value (Utilities|Struct|BreakS_ItemData _array_element)) (.value (Utilities|Struct|BreakS_ItemData (Variables|/Game/Assets/Collectibles/BP_ParentInventoryItems.BP_ParentInventoryItems_C|Getitem _asbp_parent_inventory_items)))) (.icon (Utilities|Struct|BreakS_ItemData _array_element)) (.mesh (Utilities|Struct|BreakS_ItemData _array_element))))
              (goto _label Break)
              (elif (== (.value (Utilities|Struct|BreakS_ItemData _array_element)) 0)
                (Utilities|Array|SetArrayElem (Variables|Default|GetitemDatas) _array_index (Variables|/Game/Assets/Collectibles/BP_ParentInventoryItems.BP_ParentInventoryItems_C|Getitem _asbp_parent_inventory_items))
                (goto _label Break))))
          (:Completed
            (Default|LoadInventory (Variables|Default|GetinventoryWidget) self)
            (Actor|DestroyActor _asbp_parent_inventory_items))))
      (:CastFailed
        (Development|PrintString (Utilities|GetDisplayName (.HitActor (Collision|BreakHitResult _outhit))))))))