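; Turn-based Flame Bone enemy that initializes its sprite and GAS attributes from EnemyData and binds attribute updates to its status widget.
; On its turn, UtilityAi picks a skill and target, and descriptor-built effect specs apply to itself or the target using SetByCaller magnitudes.
; When a watched attribute reaches zero, it spawns BP_EnemyRemains with random loot quantities and ash mesh, signals its death and destroys itself.
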(event Custom|Event%20On%20Disable%20Highlight)

(event Custom|Event%20On%20Enable%20Highlight)

(event Custom|Event%20On%20Attribute%20Changed
  (params (Attribute :type Gameplay%20Attribute%20Structure%20%28by%20ref%29) (CurrentValue :type Integer) (MaxValue :type Integer))
  (if (and (== Attribute "(AttributeName=\"Health\",Attribute=/Script/CS3247_Project.BasicAttributeSet:Health,AttributeOwner=\"/Script/CoreUObject.Class'/Script/CS3247_Project.BasicAttributeSet'\")") (<= CurrentValue 0))
    (CallFunction|EventonDefeated)))

(event Custom|Event%20On%20Defeated
  (bind _returnvalue (Transformation|GetActorTransform))
  (bind (_location _rotation _scale) (Math|Transform|BreakTransform _returnvalue))
  (bind _loots (CallFunction|DropLoots))
  (Game|SpawnActorfromClass "/Game/Assets/Characters/Enemies/BP_EnemyRemains.BP_EnemyRemains_C" (Math|Transform|MakeTransform (* _location "1.000000,1.000000,0.000000") _rotation _scale) "AlwaysSpawn" "MultiplyWithRoot" 0 _loots (Utilities|ResolveSoftReference (.OutItem (Utilities|Array|Random (Variables|Default|GetAshMeshes)))) 0)
  (Default|CallOnEnemyDead self)
  (Actor|DestroyActor))

(event Custom|Event%20On%20Init%20Attribute
  (params (Attribute :type Gameplay%20Attribute%20Structure) (Value :type Float%20%28double-precision%29))
  (bind _returnvalue (Ability|GetAbilitySystemComponent 0))
  (bind _asbp_dungeon_slayer_game_instance (Utilities|Casting|CastToBP_DungeonSlayerGameInstance (Game|GetGameInstance)))
  (bind _returnvalue_2 (Class|BasicGameInstance|AttributetoAssetTag _asbp_dungeon_slayer_game_instance Attribute))
  (bind _returnvalue_3 (Ability|GameplayEffect|AssignTagSetbyCallerMagnitude (GameplayEffects|MakeOutgoingSpec :self _returnvalue :GameplayEffectClass "/Game/Assets/GameplayAbilities/GameplayEffects/GE_InitAttribute.GE_InitAttribute_C" :Level 1.0) "(TagName=\"GameplayEffect.AttributeInitialisation\")" Value))
  (bind _returnvalue_4 (Ability|GameplayEffect|AddAssetTag _returnvalue_3 _returnvalue_2))
  (GameplayEffects|ApplyGameplayEffectSpecToSelf _returnvalue _returnvalue_4))

(event EventBeginPlay
  (bind _enemydata (Variables|Default|GetEnemyData))
  (bind _attributes (Variables|/Script/CS3247_Project.Enemy|GetAttributes _enemydata))
  (|CallParentFunction)
  (bind _object (Utilities|AsyncLoadAsset (Variables|/Script/CS3247_Project.Enemy|GetSprite (Variables|Default|GetEnemyData)))
    (:then
      (for _array_element (Variables|Default|GetAshMeshes)
        (Utilities|AsyncLoadAsset _array_element))
      (bind _keys (Utilities|Map|Keys _attributes))
      (for _array_element_2 _keys
        (CallFunction|EventonInitAttribute _array_element_2 (.Value (Utilities|Map|Find _attributes _array_element_2))))
      (bind _aswbp_enemy_health_display (Utilities|Casting|CastToWBP_EnemyHealthDisplay (UserInterface|GetWidget (Variables|Default|GetEnemyStatusWidget))))
      (EventDispatchers|BindEventtoOnAttributeUpdated (EventDispatchers|CreateEvent _aswbp_enemy_health_display :!event EventonAttributesUpdated))
      (EventDispatchers|BindEventtoOnAttributeUpdated (delegate Custom|Event%20On%20Attribute%20Changed)))
    (:Completed
      (bind _aspaper_sprite (Utilities|Casting|CastToPaperSprite _object))
      (Rendering|Components|Sprite|SetSprite (Variables|Default|GetSprite) _aspaper_sprite))))

(event Custom|Event%20On%20Use%20Skill
  (params (GameplayEffects :type Array%20of%20Gameplay%20Effect%20Descriptor%20Structures) (TargetCharacter :type Basic%20Character%20Object%20Reference))
  (for _array_element GameplayEffects
    (bind (_gameplayeffectspechandle _bisreflexiveeffect) (CallFunction|ToGameplayEffectSpecHandle _array_element))
    (if (or _bisreflexiveeffect (== TargetCharacter self))
      (GameplayEffects|ApplyGameplayEffectSpecToSelf (Variables|Default|GetAbilitySystemComponent) _gameplayeffectspechandle)
      (else
        (GameplayEffects|ApplyGameplayEffectSpecToTarget (Variables|Default|GetAbilitySystemComponent) _gameplayeffectspechandle (Ability|GetAbilitySystemComponent TargetCharacter))))))

(event Custom|Event%20On%20Take%20Action
  (params (Context :type Combat%20Context%20Structure))
  (bind _utilityai (Variables|Default|GetUtilityAi))
  (bind _returnvalue (Class|UtilityAiComponent|Decide _utilityai Context))
  (bind (_skilleffects _target) (Utilities|Struct|BreakAiDecision _returnvalue))
  (CallFunction|EventonUseSkill _skilleffects _target)
  (Class|BasicCharacter|SignalAllAttributeUpdates _target)
  (Class|BasicCharacter|SignalAllAttributeUpdates))

(fn ConstructionScript)

(fn DropLoots
  (for _array_element (Variables|/Script/CS3247_Project.Enemy|GetPossibleLoots (Variables|Default|GetEnemyData))
    (Utilities|Map|Add (LocalVariables|GetGeneratedLoots) (.Item (Utilities|Struct|BreakLoot _array_element)) (Math|Random|RandomIntegerinRange (.MinQuantity (Utilities|Struct|BreakLoot _array_element)) (.MaxQuantity (Utilities|Struct|BreakLoot _array_element)))))
  (return (LocalVariables|GetGeneratedLoots)))

(fn ToGameplayEffectSpecHandle
  (params (Descriptor :type Gameplay%20Effect%20Descriptor%20Structure))
  (bind _returnvalue (Ability|GameplayEffect|AssignTagSetbyCallerMagnitude (GameplayEffects|MakeOutgoingSpec :self (Ability|GetAbilitySystemComponent 0) :GameplayEffectClass (.gameplayeffecttype Descriptor) :Level 1.0) (.datatag Descriptor) (Math|Conversions|ToFloat(Integer) (.magnitude Descriptor))))
  (bind _returnvalue_2 (Ability|GameplayEffect|AddAssetTag _returnvalue (.assettag Descriptor)))
  (return _returnvalue_2 (.bisreflexive Descriptor)))