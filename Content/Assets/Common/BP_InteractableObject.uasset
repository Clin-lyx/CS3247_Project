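; BP_InteractableObject is an interactable actor, apparently a base, that shows a hint and takes input while the player is nearby.
; Collision box overlaps with BP_PlayerCharacter trigger in-range and out-of-range events.
; Entering stores the player's BP_PlayerController, sends it HintText and enables input on the actor.
; Leaving notifies the controller, disables input and clears the reference; no interaction action is defined here.
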(event OnComponentBeginOverlap(CollisionBox)
  (params (OverlappedComponent :type Primitive%20Component%20Object%20Reference) (OtherActor :type Actor%20Object%20Reference) (OtherComp :type Primitive%20Component%20Object%20Reference) (OtherBodyIndex :type Integer) (bFromSweep :type Boolean) (SweepResult :type Hit%20Result%20Structure%20%28by%20ref%29))
  (bind _asbp_player_character (Utilities|Casting|CastToBP_PlayerCharacter OtherActor))
  (Class|InteractableObject|OnPlayerinRange _asbp_player_character))

(event OnComponentEndOverlap(CollisionBox)
  (params (OverlappedComponent :type Primitive%20Component%20Object%20Reference) (OtherActor :type Actor%20Object%20Reference) (OtherComp :type Primitive%20Component%20Object%20Reference) (OtherBodyIndex :type Integer))
  (bind _asbp_player_character (Utilities|Casting|CastToBP_PlayerCharacter OtherActor))
  (Class|InteractableObject|OnPlayerOutOfRange _asbp_player_character))

(event EventOnPlayerinRange
  (params (Player :type Player%20Character%20Object%20Reference))
  (bind _asbp_player_controller (Utilities|Casting|CastToBP_PlayerController (Pawn|GetController Player)))
  (bind _output_get (Variables|Default|SetPlayerInRange _asbp_player_controller))
  (Default|EventonEnterInteractionZone _output_get (Variables|Default|GetHintText))
  (Input|EnableInput _output_get))

(event EventOnPlayerOutOfRange
  (params (Player :type Player%20Character%20Object%20Reference))
  (Default|EventonLeaveInteractionZone (Variables|Default|GetPlayerInRange))
  (Input|DisableInput (Variables|Default|GetPlayerInRange))
  (Variables|Default|SetPlayerInRange 0))

(fn ConstructionScript)