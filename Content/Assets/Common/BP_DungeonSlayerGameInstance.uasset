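; Game instance for DungeonSlayer that owns the auto-save data and exposes it through ReadSaveData.
; Loads the auto-save slot synchronously on Init and saves it synchronously on Shutdown.
; LoadGame and SaveGame also offer async paths, but only an async load fires OnGameLoaded.
; A new BP_SaveGame is created only at save time when the slot is empty, so SaveData is not populated on a first launch's Init.
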(event EventLoadGame
  (params (bIsAsync :type Boolean))
  (bind _returnvalue (SaveGame|DoesSaveGameExist (Variables|Default|GetAutoSaveSlotName)))
  (if _returnvalue
    (if bIsAsync
      (bind _savegame (|AsyncLoadGamefromSlot (Variables|Default|GetAutoSaveSlotName))
        (:Completed
          (bind _asbp_save_game (Utilities|Casting|CastToBP_SaveGame _savegame))
          (Variables|Default|SetSaveData _asbp_save_game)
          (Default|CallOnGameLoaded)))
      (else
        (bind _returnvalue_2 (SaveGame|LoadGamefromSlot (Variables|Default|GetAutoSaveSlotName)))
        (bind _asbp_save_game_2 (Utilities|Casting|CastToBP_SaveGame _returnvalue_2))
        (Variables|Default|SetSaveData _asbp_save_game_2)))))

(event EventSaveGame
  (params (bIsAsync :type Boolean))
  (bind _returnvalue (SaveGame|DoesSaveGameExist (Variables|Default|GetAutoSaveSlotName)))
  (if _returnvalue
    _
    (else
      (bind _returnvalue_2 (SaveGame|CreateSaveGameObject "/Game/SaveGames/BP_SaveGame.BP_SaveGame_C"))
      (Variables|Default|SetSaveData _returnvalue_2)))
  (if bIsAsync
    (|AsyncSaveGametoSlot (Variables|Default|GetSaveData) (Variables|Default|GetAutoSaveSlotName))
    (else
      (SaveGame|SaveGametoSlot (Variables|Default|GetSaveData) (Variables|Default|GetAutoSaveSlotName)))))

(event EventInit
  (CallFunction|LoadGame false))

(event EventShutdown
  (CallFunction|SaveGame false))

(fn ReadSaveData
  (return (Variables|Default|GetSaveData)))